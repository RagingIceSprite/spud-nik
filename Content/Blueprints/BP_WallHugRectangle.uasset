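; Wall-hug volume that turns on hugging for a ThirdPersonDemoCharacter entering its box.
; The construction script sizes the box and builds a rounded-rectangle spline from size and border radius.
; On overlap it stores the character's closest distance along the spline, interpolated between spline points, and draws a debug point there.
; End-overlap and GetNextPosition are empty, with turn-off and movement-along-spline logic left disconnected.
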(event `self.Box.OnComponentBeginOverlap`
  (params (OverlappedComponent :type "PrimitiveComponent Object Reference") (OtherActor :type "Actor Object Reference") (OtherComp :type "PrimitiveComponent Object Reference") (OtherBodyIndex :type Integer) (bFromSweep :type Boolean) (SweepResult :type "HitResult Structure (by ref)"))
  (bind _spline (`self.Spline`))
  (bind _asthird_person_demo_character (cast `/Game/Assets/Blueprints/ThirdPersonDemoCharacter` OtherActor))
  (`/Game/Assets/Blueprints/ThirdPersonDemoCharacter.TurnOnHug` _asthird_person_demo_character self)
  (bind _output_get (set `self.PlayerDistance` (`self.FindDistanceAlongSplineClosestToWorldLocation` (`self.K2_GetActorLocation` _asthird_person_demo_character) _spline)))
  (`KismetSystemLibrary.DrawDebugPoint` (`SplineComponent.GetLocationAtDistanceAlongSpline` _spline _output_get "World") 45.0 (struct :`R` 1.0 :`G` 0.897106 :`A` 1.0) 15.0))

(event `self.Box.OnComponentEndOverlap`
  (params (OverlappedComponent :type "PrimitiveComponent Object Reference") (OtherActor :type "Actor Object Reference") (OtherComp :type "PrimitiveComponent Object Reference") (OtherBodyIndex :type Integer)))

(fn `FindDistanceAlongSplineClosestToWorldLocation`
  (params (Location :type "Vector Structure") (Spline :type "SplineComponent Object Reference"))
  (returns (Distance :type "Float (double-precision)"))
  (bind _returnvalue (`SplineComponent.FindInputKeyClosestToWorldLocation` Spline Location))
  (bind _returnvalue_2 (`KismetMathLibrary.FTrunc` _returnvalue))
  (bind _returnvalue_3 (`SplineComponent.GetDistanceAlongSplineAtSplinePoint` Spline _returnvalue_2))
  (return (+ _returnvalue_3 (* (- (`SplineComponent.GetDistanceAlongSplineAtSplinePoint` Spline (`KismetMathLibrary.FTrunc` (+ _returnvalue 1.0))) _returnvalue_3) (- _returnvalue (`KismetMathLibrary.Conv_IntToDouble` _returnvalue_2))))))

(fn `GetNextPosition`
  (params (HorizontalValue :type "Float (double-precision)") (VerticalValue :type "Float (double-precision)") (Speed :type "Float (double-precision)"))
  (returns (Position :type "Vector Structure"))
  (locals (Result :type "Vector Structure") (NextDistance :type "Float (double-precision)")))

(fn `UserConstructionScript`
  (bind _spline (`self.Spline`))
  (bind (_splinepoints _tangentpoints) (`WallHugSpline.MakeRectangleSpline` (`self.xSize`) (`self.ySize`) (`self.borderRadius`)))
  (`BoxComponent.SetBoxExtent` (`self.Box`) (`KismetMathLibrary.MakeVector` (`self.boxX`) (`self.boxY`) (`self.boxZ`)) true)
  (`SplineComponent.ClearSplinePoints` (`self.Spline`) false)
  (for _array_element _splinepoints
    (`SplineComponent.AddSplinePoint` _spline _array_element "Local" false))
  (for (_array_element_2 _array_index) _tangentpoints
    (`SplineComponent.SetTangentAtSplinePoint` _spline _array_index _array_element_2 "Local" true))
  (set `SplineComponent.bInputSplinePointsToConstructionScript` true _spline))