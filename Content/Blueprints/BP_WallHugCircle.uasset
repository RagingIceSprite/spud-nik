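; BP_WallHugCircle is an actor that pairs a resizable box with a circular spline, apparently for wall-hugging as its name suggests.
; The construction script sizes the box from per-axis variables, then rebuilds the spline in local space using points and tangents that MakeCircleSpline generates from Radius.
; It holds no active runtime logic, and GetTangent is a stub returning a zero vector.
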(fn `GetTangent`
  (returns (Tangent :type "Vector Structure"))
  (return (0.0 0.0 0.0)))

(fn `UserConstructionScript`
  (bind _spline (`self.Spline`))
  (bind (_splinepoints _tangentpoints) (`WallHugSpline.MakeCircleSpline` (`self.radius`)))
  (`BoxComponent.SetBoxExtent` (`self.Box`) (`KismetMathLibrary.MakeVector` (`self.boxX`) (`self.boxY`) (`self.boxZ`)) true)
  (`SplineComponent.ClearSplinePoints` (`self.Spline`) false)
  (for _array_element _splinepoints
    (`SplineComponent.AddSplinePoint` _spline _array_element "Local" false))
  (for (_array_element_2 _array_index) _tangentpoints
    (`SplineComponent.SetTangentAtSplinePoint` _spline _array_index _array_element_2 "Local" true))
  (set `SplineComponent.bInputSplinePointsToConstructionScript` true _spline))