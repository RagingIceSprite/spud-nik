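; SliderDot is a marker actor that tracks the position of a Plat_OSC platform in the level.
; Each Tick it reads StopPressed from the ThirdPersonDemoCharacter player and hides itself while that flag is set.
; Otherwise it shows itself and snaps to the PlatformBase world location of the first Plat_OSC found, repeating the GetAllActorsOfClass search on every such frame.
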(event `self.ReceiveTick`
  (params (DeltaSeconds :type "Float (single-precision)"))
  (bind _asthird_person_demo_character (cast `/Game/Assets/Blueprints/ThirdPersonDemoCharacter` (`GameplayStatics.GetPlayerCharacter` 0)))
  (if (`/Game/Assets/Blueprints/ThirdPersonDemoCharacter.StopPressed` _asthird_person_demo_character)
    (`self.SetActorHiddenInGame` true)
    (else
      (`self.SetActorHiddenInGame` false)
      (bind _outactors (`GameplayStatics.GetAllActorsOfClass` "/Game/Blueprints/Plat_OSC.Plat_OSC_C"))
      (`self.K2_SetActorLocation` (`SceneComponent.K2_GetComponentLocation` (`/Game/Blueprints/Plat_OSC.PlatformBase` (`|GetArrayItem` _outactors)))))))

(fn `UserConstructionScript`)