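; Oscillating platform actor that moves its PlatformBase back and forth between Start and End points.
; Every Tick it sets the base's world location by interpolating between the two points with a game-time sine wave, slowed by TimeScaleInverse.
; The actor destroys itself once the player's FirstPersonCharacter has StopPressed set.
; Its overlap and hit events are empty, and the unpause and extra destroy chains are unconnected.
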(event `self.ReceiveTick`
  (params (DeltaSeconds :type "Float (single-precision)"))
  (bind _returnvalue_location (`KismetMathLibrary.BreakTransform` (`KismetMathLibrary.TLerp` (`KismetMathLibrary.MakeTransform` (`SceneComponent.K2_GetComponentLocation` (`self.Start`))) (`KismetMathLibrary.MakeTransform` (`SceneComponent.K2_GetComponentLocation` (`self.End`))) (/ (+ (`KismetMathLibrary.Sin` (/ (`KismetSystemLibrary.GetGameTimeInSeconds`) (`self.TimeScaleInverse`))) 1.0) 2.0))))
  (bind _asfirst_person_character (cast `/Game/FirstPersonCPP/Blueprints/FirstPersonCharacter` (`GameplayStatics.GetPlayerCharacter` 0)))
  (if (`/Game/FirstPersonCPP/Blueprints/FirstPersonCharacter.StopPressed` _asfirst_person_character)
    (`self.K2_DestroyActor`)
    (else
      (`SceneComponent.K2_SetWorldLocation` (`self.PlatformBase`) _returnvalue_location false false))))

(event `self.SliderRange1.OnComponentBeginOverlap`
  (params (OverlappedComponent :type "PrimitiveComponent Object Reference") (OtherActor :type "Actor Object Reference") (OtherComp :type "PrimitiveComponent Object Reference") (OtherBodyIndex :type Integer) (bFromSweep :type Boolean) (SweepResult :type "HitResult Structure (by ref)")))

(event `self.PlatformBase.OnComponentBeginOverlap`
  (params (OverlappedComponent :type "PrimitiveComponent Object Reference") (OtherActor :type "Actor Object Reference") (OtherComp :type "PrimitiveComponent Object Reference") (OtherBodyIndex :type Integer) (bFromSweep :type Boolean) (SweepResult :type "HitResult Structure (by ref)")))

(event `self.SliderRange1.OnComponentHit`
  (params (HitComponent :type "PrimitiveComponent Object Reference") (OtherActor :type "Actor Object Reference") (OtherComp :type "PrimitiveComponent Object Reference") (NormalImpulse :type "Vector Structure") (Hit :type "HitResult Structure (by ref)")))

(fn `UserConstructionScript`)