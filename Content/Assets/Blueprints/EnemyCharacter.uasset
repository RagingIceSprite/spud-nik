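; Enemy character that patrols between points and displays its field of view as a vision cone mesh.
; Every Tick runs an EQS query, whose result locations become actor-relative vertices of a procedural triangle fan, with world rotation zeroed.
; Helper functions cycle patrol points, set walk speed and switch the cone between default, warning and alert materials.
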(event `self.ReceiveBeginPlay`
  (bind _numberofpoints (`self.NumberOfPoints`))
  (`KismetArrayLibrary.Array_Resize` (`self.Vertices`) (+ _numberofpoints 1))
  (`KismetArrayLibrary.Array_Resize` (`self.Triangles`) (* _numberofpoints 3)))

(event `self.ReceiveTick`
  (params (DeltaSeconds :type "Float (single-precision)"))
  (bind _returnvalue (`EnvQueryManager.RunEQSQuery` "/Game/Assets/Blueprints/AI/VisionCone.VisionCone" self "AllMatching"))
  (add `EnvQueryInstanceBlueprintWrapper.OnQueryFinishedEvent` _returnvalue (delegate `MakeCone`)))

(event `MakeCone`
  (params (QueryInstance :type "EnvQueryInstanceBlueprintWrapper Object Reference") (QueryStatus :type "EEnvQueryStatus Enum" :default "Processing"))
  (bind _resultlocations (`EnvQueryInstanceBlueprintWrapper.GetQueryResultsAsLocations` QueryInstance))
  (bind _output_get (set `self.SightPoints` _resultlocations))
  (bind (_vertices _triangles) (`self.ConvertSightToVertices` _output_get))
  (`self.MakeViewCone` _vertices _triangles))

(fn `ConvertSightToVertices`
  (params (SightPoints :type "Array of Vector Structure"))
  (returns (Vertices :type "Array of Vector Structure") (Triangles :type "Array of Integer"))
  (bind (_returnvalue_x _returnvalue_y) (`KismetMathLibrary.BreakVector` (`self.K2_GetActorLocation`)))
  (`KismetArrayLibrary.Array_Set` (`self.Vertices`))
  (for (_array_element _array_index) SightPoints
    (`KismetArrayLibrary.Array_Set` (`self.Vertices`) (+ _array_index 1) (`KismetMathLibrary.MakeVector` (- (.x _array_element) _returnvalue_x) (- (.y _array_element) _returnvalue_y) (`self.ConeHeight`))))
  (for _index (range (+ (`KismetArrayLibrary.Array_Length` (`self.Vertices`)) 1))
    (bind _returnvalue (* _index 3))
    (`KismetArrayLibrary.Array_Set` (`self.Triangles`) _returnvalue)
    (bind _returnvalue_2 (+ _returnvalue 1))
    (bind _returnvalue_3 (+ _index 1))
    (`KismetArrayLibrary.Array_Set` (`self.Triangles`) _returnvalue_2 _returnvalue_3)
    (`KismetArrayLibrary.Array_Set` (`self.Triangles`) (+ _returnvalue_2 1) (+ _returnvalue_3 1)))
  (return (`self.Vertices`) (`self.Triangles`)))

(fn `GetCurrentSpot`
  (returns (Location :type "Vector Structure"))
  (return (`self.K2_GetActorLocation` (`|GetArrayItem` (`self.PatrolPoints`) (`self.PatrolSpotIdx`)))))

(fn `GetNextSpot`
  (returns (Location :type "Vector Structure"))
  (bind _patrolpoints (`self.PatrolPoints`))
  (bind _output_get (set `self.PatrolSpotIdx` (mod (+ (`self.PatrolSpotIdx`) 1) (`KismetArrayLibrary.Array_Length` _patrolpoints))))
  (return (`self.K2_GetActorLocation` (`|GetArrayItem` _patrolpoints _output_get))))

(fn `MakeViewCone`
  (params (Vertices :type "Array of Vector Structure") (Triangles :type "Array of Integer"))
  (bind _visioncone (`self.VisionCone`))
  (`ProceduralMeshComponent.CreateMeshSection_LinearColor` :`self` _visioncone :`Vertices` Vertices :`Triangles` Triangles)
  (`PrimitiveComponent.SetMaterial` _visioncone 0 (`self.CurrentMaterial`))
  (`SceneComponent.K2_SetWorldRotation` :`self` _visioncone))

(fn `SetAlertMaterial`
  (set `self.CurrentMaterial` (`self.AlertMaterial`)))

(fn `SetDefaultMaterial`
  (set `self.CurrentMaterial` (`self.DefaultMaterial`)))

(fn `SetWalkingSpeed`
  (params (speed :type "Float (double-precision)"))
  (set `CharacterMovementComponent.MaxWalkSpeed` speed (`self.CharacterMovement`)))

(fn `SetWarningMaterial`
  (set `self.CurrentMaterial` (`self.WarningMaterial`)))

(fn `UserConstructionScript`)