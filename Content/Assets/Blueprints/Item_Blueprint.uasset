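; Pickup item, the farm tools, that attaches to the third-person demo character when it overlaps the item's box.
; The overlap snaps it to a socket on a character component, shows a HUD message pointing to the farm, flags ItemAttached on the game mode and becomes the character's CurrentItem.
; End overlap clears the text but reruns the same HUD, game mode and CurrentItem chain.
; BeginPlay records the start location.
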(event `self.ReceiveBeginPlay`
  (set `self.StartPoint` (`self.K2_GetActorLocation`)))

(event `self.Box.OnComponentBeginOverlap`
  (params (OverlappedComponent :type "PrimitiveComponent Object Reference") (OtherActor :type "Actor Object Reference") (OtherComp :type "PrimitiveComponent Object Reference") (OtherBodyIndex :type Integer) (bFromSweep :type Boolean) (SweepResult :type "HitResult Structure (by ref)"))
  (bind _asthird_person_demo_character (cast `/Game/Assets/Blueprints/ThirdPersonDemoCharacter` OtherActor))
  (`self.K2_AttachToComponent` (`/Game/Assets/Blueprints/ThirdPersonDemoCharacter.NewVar_1` _asthird_person_demo_character) "Socket" "SnapToTarget" "SnapToTarget" "SnapToTarget")
  (set `self.Text` "Tools obtained! Head to the farm!")
  (bind _asdemo_hud (cast `/Game/Assets/Blueprints/DemoHud` (`PlayerController.GetHUD` (`GameplayStatics.GetPlayerController` 0)) :!label _label))
  (`/Game/Assets/Blueprints/DemoHud.Draw Text to Screen` _asdemo_hud true (`self.Text`))
  (bind _astech_prototype_demo (cast `/Game/Assets/Blueprints/TechPrototypeDemo` (`GameplayStatics.GetGameMode`)))
  (set `/Game/Assets/Blueprints/TechPrototypeDemo.Item Attached` true _astech_prototype_demo)
  (set `/Game/Assets/Blueprints/ThirdPersonDemoCharacter.CurrentItem` self _asthird_person_demo_character))

(event `self.ReceiveActorEndOverlap`
  (params (OtherActor :type "Actor Object Reference"))
  (set `self.Text` "")
  (goto _label))

(fn `UserConstructionScript`)