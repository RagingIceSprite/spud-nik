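; Test actor for spline direction math that traces a circular spline and visualises it with debug drawing.
; The construction script builds four points at Radius, with tangents scaled by a constant derived from the Bézier circle approximation.
; BeginPlay places Cube at the spline start.
; Tick advances a looping distance at constant speed, draws that point and direction, and prints the direction's 2D cosine against an adjustable debug vector.
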(event EventBeginPlay
  (Variables|Default|SetDebugVector (Math|Vector|MakeVector (Variables|Default|GetDebugx) (Variables|Default|GetDebugY) 0.0))
  (Transformation|SetWorldLocation (Variables|Default|GetCube) (Spline|GetLocationatDistanceAlongSpline (Variables|Default|GetSpline) 0.0 "World") false false))

(event Collision|EventActorBeginOverlap
  (params (OtherActor :type Actor%20Object%20Reference)))

(event EventTick
  (params (DeltaSeconds :type Float%20%28single-precision%29))
  (bind _spline (Variables|Default|GetSpline))
  (bind _returnvalue (Spline|GetSplineLength _spline))
  (Rendering|Debug|DrawDebugArrow "0.0,0.0,0.0" (* (Math|Vector|Normalize (Variables|Default|GetDebugVector)) 75.0) 1e+01 "(R=0.000000,G=1.000000,B=0.577141,A=1.000000)" 0.02 3.0)
  (if (> (+ (* DeltaSeconds 1.3e+02) (Variables|Default|GetDistanceT)) _returnvalue)
    (Variables|Default|SetDistanceT (- (Variables|Default|GetDistanceT) _returnvalue))
    (else
      (Variables|Default|SetDistanceT (+ (* DeltaSeconds 1.3e+02) (Variables|Default|GetDistanceT)))))
  (Rendering|Debug|DrawDebugArrow (Spline|GetDirectionatDistanceAlongSpline (Variables|Default|GetSpline) (Variables|Default|GetDistanceT) "Local") (* (Spline|GetDirectionatDistanceAlongSpline (Variables|Default|GetSpline) (Variables|Default|GetDistanceT) "Local") 3e+01) 1e+01 "(R=0.000000,G=0.848958,B=0.848958,A=1.000000)" 0.02 3.0)
  (Rendering|Debug|DrawDebugPoint (Spline|GetLocationatDistanceAlongSpline (Variables|Default|GetSpline) (Variables|Default|GetDistanceT) "World") 1e+01 "(R=0.765625,G=0.387382,B=0.000000,A=1.000000)" 0.02)
  (Development|PrintString (Utilities|String|ToString(Float) (Class|KismetMathLibrary|VectorCosineAngle2D (Spline|GetDirectionatDistanceAlongSpline (Variables|Default|GetSpline) (Variables|Default|GetDistanceT) "Local") (Variables|Default|GetDebugVector))) true false "(R=1.000000,G=0.867966,B=0.020612,A=1.000000)" 0.02))

(event Input|AxisEvents|InputAxisMoveForwardandBack
  (params (AxisValue :type Float%20%28single-precision%29))
  (if true
    _))

(event Input|AxisEvents|InputAxisMoveLeftandRight
  (params (AxisValue :type Float%20%28single-precision%29)))

(fn ConstructionScript
  (bind _spline (Variables|Default|GetSpline))
  (bind _radius (Variables|Default|GetRadius))
  (bind _radius_2 (Variables|Default|GetRadius))
  (bind _spline_2 (Variables|Default|GetSpline))
  (bind _spline_3 (Variables|Default|GetSpline))
  (bind _returnvalue (* _radius_2 -1.0))
  (Spline|ClearSplinePoints _spline false)
  (Spline|AddSplinePoint _spline (Math|Vector|MakeVector _radius 0.0 0.0) "Local" false)
  (Spline|AddSplinePoint _spline (Math|Vector|MakeVector 0.0 _radius 0.0) "Local" false)
  (Spline|AddSplinePoint _spline_2 (Math|Vector|MakeVector _returnvalue 0.0 0.0) "Local" false)
  (Spline|AddSplinePoint _spline_2 (Math|Vector|MakeVector 0.0 _returnvalue 0.0) "Local" false)
  (Variables|Default|SetCircleConst (+ (|((4*((sqrt(2))-1))/3)) 1.0))
  (for _index (range 0 (Spline|GetNumberOfSplinePoints (Variables|Default|GetSpline)))
    (switch int _index
      (:0
        (Spline|SetTangentatSplinePoint _spline_3 _index (Math|Vector|MakeVector 0.0 (* (Variables|Default|GetRadius) (Variables|Default|GetCircleConst) 1.0) 0.0) "Local" true))
      (:1
        (Spline|SetTangentatSplinePoint _spline_3 _index (Math|Vector|MakeVector (* (Variables|Default|GetRadius) (Variables|Default|GetCircleConst) -1.0) 0.0 0.0) "Local" false))
      (:2
        (Spline|SetTangentatSplinePoint _spline_3 _index (Math|Vector|MakeVector 0.0 (* (Variables|Default|GetRadius) (Variables|Default|GetCircleConst) -1.0) 0.0) "Local" false))
      (:3
        (Spline|SetTangentatSplinePoint _spline_3 _index (Math|Vector|MakeVector (* (Variables|Default|GetRadius) (Variables|Default|GetCircleConst) 1.0) 0.0 0.0) "Local" false))))
  (Variables|/Script/Engine.SplineComponent|SetbInputSplinePointsToConstructionScript _spline_3 true))