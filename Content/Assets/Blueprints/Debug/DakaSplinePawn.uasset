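; Debug pawn that tests moving a cube along a spline using 2D axis input.
; The construction script builds a rounded-rectangle spline.
; Each tick, when input direction is within an angle tolerance of the spline tangent at the cube, GetNextDistance steps it in reverse with wraparound.
; Tick also draws arrows for input, tangents and a debug vector, animates a looping sample point, and prints angle readouts.
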(event `self.ReceiveBeginPlay`
  (set `self.DebugVector` (`KismetMathLibrary.MakeVector` (`self.Debugx`) (`self.DebugY`)))
  (`SceneComponent.K2_SetWorldLocation` (`self.Cube`) (`SplineComponent.GetLocationAtDistanceAlongSpline` (`self.Spline`) 0.0 "World") false false))

(event `self.ReceiveTick`
  (params (DeltaSeconds :type "Float (single-precision)"))
  (bind _returnvalue (`self.K2_GetActorLocation`))
  (bind _returnvalue_2 (`self.K2_GetActorLocation`))
  (bind _returnvalue_3 (`self.K2_GetActorLocation`))
  (bind _returnvalue_4 (`SplineComponent.GetDirectionAtDistanceAlongSpline` (`self.Spline`) (`self.DebugDistance`) "World"))
  (bind _returnvalue_5 (`SplineComponent.GetDirectionAtDistanceAlongSpline` (`self.Spline`) (`self.DistanceT`) "World"))
  (bind _returnvalue_6 (`SplineComponent.GetSplineLength` (`self.Spline`)))
  (bind _returnvalue_7 (+ (* DeltaSeconds 70.0) (`self.DistanceT`)))
  (bind _returnvalue_8 (`KismetMathLibrary.Normal` (`KismetMathLibrary.MakeVector` (`self.GetInputAxisValue`) (`self.GetInputAxisValue`))))
  (bind _returnvalue_9 (`KismetMathLibrary.DegAcos` (`KismetMathLibrary.Vector_CosineAngle2D` _returnvalue_8 _returnvalue_4)))
  (`KismetSystemLibrary.DrawDebugArrow` _returnvalue_3 (+ _returnvalue_3 (* (`KismetMathLibrary.Normal` (`self.DebugVector`)) 75.0)) 10.0 (struct :`G` 1.0 :`B` 0.577141 :`A` 1.0) 0.02 3.0)
  (if (> _returnvalue_7 _returnvalue_6)
    (set `self.DistanceT` (- (`self.DistanceT`) _returnvalue_6))
    (else
      (set `self.DistanceT` _returnvalue_7)))
  (`KismetSystemLibrary.DrawDebugArrow` _returnvalue (+ _returnvalue (* _returnvalue_5 30.0)) 10.0 (struct :`G` 0.848958 :`B` 0.848958 :`A` 1.0) 0.02 3.0)
  (`KismetSystemLibrary.DrawDebugPoint` (`SplineComponent.GetLocationAtDistanceAlongSpline` (`self.Spline`) (`self.DistanceT`) "World") 10.0 (struct :`R` 0.765625 :`G` 0.387382 :`A` 1.0) 0.02)
  (`KismetSystemLibrary.PrintString` (`KismetStringLibrary.Conv_DoubleToString` (`KismetMathLibrary.Vector_CosineAngle2D` _returnvalue_5 (`self.DebugVector`))) true false (struct :`R` 1.0 :`G` 0.867966 :`B` 0.020612 :`A` 1.0) 0.02)
  (`KismetSystemLibrary.DrawDebugArrow` _returnvalue_2 (+ _returnvalue_2 (* _returnvalue_8 100.0)) 10.0 (struct :`R` 1.0 :`G` 0.989155 :`A` 1.0) 0.02 3.0)
  (`KismetSystemLibrary.DrawDebugArrow` _returnvalue_2 (+ _returnvalue_2 (* _returnvalue_4 100.0)) 10.0 (struct :`R` 1.0 :`B` 0.307249 :`A` 1.0) 0.02 3.0)
  (`KismetSystemLibrary.PrintString` (`KismetStringLibrary.Conv_DoubleToString` _returnvalue_9) true false (struct :`G` 1.0 :`B` 0.153675 :`A` 1.0) 0.02)
  (if (<= _returnvalue_9 (`self.DebugAngleTolerance`))
    (bind _distance (`self.GetNextDistance` true (`KismetMathLibrary.VSize` _returnvalue_8)))
    (bind _output_get (set `self.DebugDistance` _distance))
    (`SceneComponent.K2_SetWorldLocation` (`self.Cube`) (`SplineComponent.GetLocationAtDistanceAlongSpline` (`self.Spline`) _output_get "World") false false)))

(event `InputAxis|MoveForwardandBack`
  (params (AxisValue :type "Float (single-precision)")))

(event `InputAxis|MoveLeftandRight`
  (params (AxisValue :type "Float (single-precision)")))

(fn `GetNextDistance`
  (params (Reverse :type Boolean) (input :type "Float (double-precision)"))
  (returns (Distance :type "Float (double-precision)"))
  (locals (Multiplier :type "Float (double-precision)") (NextDistance :type "Float (double-precision)"))
  (if Reverse
    (set `local.Multiplier` -1.0)
    (else
      (set `local.Multiplier` 1.0)))
  (bind _result (`self.WrapAround` (+ (`self.DebugDistance`) (* (* (`GameplayStatics.GetWorldDeltaSeconds`) 220.0) (`local.Multiplier`) input)) 0.0 (`SplineComponent.GetSplineLength` (`self.Spline`))))
  (bind _output_get (set `local.NextDistance` _result))
  (return _output_get))

(fn `UserConstructionScript`
  (bind _spline (`self.Spline`))
  (bind (_splinepoints _tangentpoints) (`WallHugSpline.MakeRectangleSpline` (`self.boxX`) (`self.boxY`) (`self.borderRadius`)))
  (`SplineComponent.ClearSplinePoints` _spline false)
  (for _array_element _splinepoints
    (`SplineComponent.AddSplinePoint` _spline _array_element "Local" false))
  (for (_array_element_2 _array_index) _tangentpoints
    (`SplineComponent.SetTangentAtSplinePoint` _spline _array_index _array_element_2 "Local" true))
  (set `SplineComponent.bInputSplinePointsToConstructionScript` true (`self.Spline`)))

(fn `WrapAround`
  (params (Value :type "Float (double-precision)") (Min :type "Float (double-precision)") (Max :type "Float (double-precision)"))
  (returns (Result :type "Float (double-precision)"))
  (locals (Temp :type "Float (double-precision)"))
  (if (> Value Max)
    (set `local.Temp` (- Value Max))
    (elif (< Value Min)
      (set `local.Temp` (- Max Value))
      (else
        (set `local.Temp` Value))))
  (return (`local.Temp`)))