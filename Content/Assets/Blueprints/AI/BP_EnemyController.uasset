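; AI controller for enemies that runs BT_Enemy on possession and reacts to perceived players and projectiles.
; Perception updates write CanSeePlayer, SawRock and TargetActor to the Blackboard while switching the enemy's material between alert, warning and default.
; A sensed player triggers alert, other character updates clear it, and a sensed projectile triggers warning.
; FinishScanning restores the default material and clears SawRock.
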(event `self.ReceivePossess`
  (params (PossessedPawn :type "Pawn Object Reference"))
  (`self.RunBehaviorTree` "/Game/Assets/Blueprints/AI/BT_Enemy.BT_Enemy"))

(event `self.AIPerception.OnTargetPerceptionUpdated`
  (params (Actor :type "Actor Object Reference") (Stimulus :type "AIStimulus Structure"))
  (bind ((`bSuccessfullySensed` _bsuccessfullysensed)) (break `AIStimulus` Stimulus))
  (bind _blackboard (`self.Blackboard`))
  (bind _blackboard_2 (`self.Blackboard`))
  (bind _ascharacter (cast `Character` Actor)
    (:`then`
      (if (and (`Pawn.IsPlayerControlled` _ascharacter) _bsuccessfullysensed)
        (bind _asenemy_character (cast `/Game/Assets/Blueprints/EnemyCharacter` (`self.K2_GetPawn`)))
        (`/Game/Assets/Blueprints/EnemyCharacter.SetAlertMaterial` _asenemy_character)
        (`BlackboardComponent.SetValueAsBool` _blackboard "CanSeePlayer" true)
        (`BlackboardComponent.SetValueAsObject` _blackboard "TargetActor" Actor)
        (else
          (`/Game/Assets/Blueprints/EnemyCharacter.SetDefaultMaterial` _asenemy_character)
          (`BlackboardComponent.SetValueAsBool` _blackboard "CanSeePlayer" false))))
    (:`CastFailed`
      (bind _asprojectile (cast `/Game/Assets/Blueprints/Projectile` Actor))
      (if _bsuccessfullysensed
        (bind _asenemy_character_2 (cast `/Game/Assets/Blueprints/EnemyCharacter` (`self.K2_GetPawn`)))
        (`/Game/Assets/Blueprints/EnemyCharacter.SetWarningMaterial` _asenemy_character_2)
        (`BlackboardComponent.SetValueAsObject` _blackboard_2 "TargetActor" _asprojectile)
        (`BlackboardComponent.SetValueAsBool` _blackboard_2 "SawRock" true)))))

(fn `FinishScanning`
  (bind _asenemy_character (cast `/Game/Assets/Blueprints/EnemyCharacter` (`self.K2_GetPawn` self)))
  (`/Game/Assets/Blueprints/EnemyCharacter.SetDefaultMaterial` _asenemy_character)
  (`BlackboardComponent.SetValueAsBool` (`self.Blackboard`) "SawRock" false))

(fn `UserConstructionScript`)